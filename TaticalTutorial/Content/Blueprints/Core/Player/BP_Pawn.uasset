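; BP_Pawn is a camera pawn that the player moves, zooms and rotates.
; Enhanced Input actions update desired targets: WASD shifts location along the actor's forward and right vectors, the mouse wheel sets a clamped spring arm length, and Q/E adds a yaw step on press.
; Tick interpolates location, rotation and arm length toward those targets for smooth motion, without sweeping for collision.
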(event Input|EnhancedActionEvents|EnhancedInputActionIA_ZoomCamera
  (params (ActionValue :type Float%20%28double-precision%29) (ElapsedSeconds :type Float%20%28double-precision%29) (TriggeredSeconds :type Float%20%28double-precision%29) (InputAction :type Input%20Action%20Object%20Reference :default "/Game/Blueprints/Core/Player/IA_ZoomCamera.IA_ZoomCamera"))
  ;[1 1 1] Zoom Camera - Mouse Wheel
  (Variables|Default|SetZoomDesired (Math|Float|Clamp(Float) (+ (Variables|Default|GetZoomDesired) (* ActionValue (Variables|Default|GetZoomSpeed))) (Variables|Default|GetZoomMin) (Variables|Default|GetZoomMax))))

(event Input|EnhancedActionEvents|EnhancedInputActionIA_MoveCamera
  (params (ActionValue :type Vector%202D%20Structure) (ElapsedSeconds :type Float%20%28double-precision%29) (TriggeredSeconds :type Float%20%28double-precision%29) (InputAction :type Input%20Action%20Object%20Reference :default "/Game/Blueprints/Core/Player/IA_MoveCamera.IA_MoveCamera"))
  ;[1 1 1] Move Camera - WASD
  (bind _output_get (Variables|Default|SetLocationDesired (+ (Variables|Default|GetLocationDesired) (* (* (.x ActionValue) (Variables|Default|GetLocationSpeed)) (Transformation|GetActorForwardVector)))))
  (Variables|Default|SetLocationDesired (+ _output_get (* (* (.y ActionValue) (Variables|Default|GetLocationSpeed)) (Transformation|GetActorRightVector)))))

(event Input|EnhancedActionEvents|EnhancedInputActionIA_RotateCamera
  (params (ActionValue :type Float%20%28double-precision%29) (ElapsedSeconds :type Float%20%28double-precision%29) (TriggeredSeconds :type Float%20%28double-precision%29) (InputAction :type Input%20Action%20Object%20Reference :default "/Game/Blueprints/Core/Player/IA_RotateCamera.IA_RotateCamera"))
  ;[1 1 1] Rotate Camera - E Q
  (:Started
    (Variables|Default|SetRotationDesired (Math|Rotator|CombineRotators (Variables|Default|GetRotationDesired) (Math|Rotator|MakeRotator 0.0 0.0 (* ActionValue (Variables|Default|GetRotationSpeed)))))))

(event EventBeginPlay
  (Variables|Default|SetLocationDesired (Transformation|GetActorLocation))
  (Variables|Default|SetZoomDesired (Variables|/Script/Engine.SpringArmComponent|GetTargetArmLength (Variables|Default|GetSpringArm)))
  (Variables|Default|SetRotationDesired (Transformation|GetActorRotation)))

(event EventTick
  (params (DeltaSeconds :type Float%20%28single-precision%29))
  (bind _springarm (Variables|Default|GetSpringArm))
  ;[1 1 1] Movement of the camera - Smoth using interpolation
  (Variables|/Script/Engine.SpringArmComponent|SetTargetArmLength _springarm (Math|Interpolation|FInterpTo (Variables|/Script/Engine.SpringArmComponent|GetTargetArmLength _springarm) (Variables|Default|GetZoomDesired) (Utilities|Time|GetWorldDeltaSeconds) (Variables|Default|GetZoomInterp)))
  (Transformation|SetActorLocation (Math|Interpolation|VInterpTo (Transformation|GetActorLocation) (Variables|Default|GetLocationDesired) (Utilities|Time|GetWorldDeltaSeconds) (Variables|Default|GetLocationInterp)) false false)
  (Transformation|SetActorRotation (Math|Interpolation|RInterpTo (Transformation|GetActorRotation) (Variables|Default|GetRotationDesired) (Utilities|Time|GetWorldDeltaSeconds) (Variables|Default|GetRotationInterp))))

(fn ConstructionScript)