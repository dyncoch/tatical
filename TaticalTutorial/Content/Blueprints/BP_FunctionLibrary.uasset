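; Blueprint function library of small debug and math helpers.
; PrintError shows a titled error message on screen in red.
; SnapVectorToVector grid-snaps each axis of one vector using the matching component of the second as grid size, and prints inputs and result on every call.
; IsFloatEven tests whether a float modulo two equals zero.
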(fn PrintError
  (params (Title :type String) (Error :type String))
  (Development|PrintString 0 (Utilities|String|Append "Error - " Title " - " Error) true true "(R=1.000000,G=0.000000,B=0.023146,A=1.000000)" 1e+01))

(fn SnapVectortoVector
  (params (V1 :type Vector) (V2 :type Vector))
  (bind (_x _y _z) (Math|Vector|BreakVector V1))
  (bind (_x_2 _y_2 _z_2) (Math|Vector|BreakVector V2))
  (bind _returnvalue (Math|Float|SnapToGrid(Float) _z _z_2))
  (bind _returnvalue_2 (Math|Float|SnapToGrid(Float) _x _x_2))
  (bind _returnvalue_3 (Math|Float|SnapToGrid(Float) _y _y_2))
  (bind _returnvalue_4 (Math|Vector|MakeVector _returnvalue_2 _returnvalue_3 _returnvalue))
  (Development|PrintString 0 (Utilities|String|Append "V1 = " (Utilities|String|ToString(Vector) V1) " | " "V2 = " (Utilities|String|ToString(Vector) V2) " | " "Return = " (Utilities|String|ToString(Vector) _returnvalue_4)) true true "(R=0.000000,G=0.660000,B=1.000000,A=1.000000)" 1e+01)
  (return _returnvalue_4))

(fn IsFloatEven
  (params (Fload :type Float%20%28double-precision%29))
  (return (== (Math|Float|%(Float) Fload 2.0) 0.0)))